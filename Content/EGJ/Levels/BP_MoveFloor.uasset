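; BP_MoveFloor is a moving floor actor that travels back and forth along the world X axis in a level.
; Each Tick it offsets itself by a Speed vector without sweep, then flips that vector when its X position passes hardcoded bounds.
; The backward velocity comes from the ReturnSpeed variable, while the forward one is hardcoded.
; Movement is per frame and not scaled by delta time, so it depends on frame rate.
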(event EventBeginPlay)

(event Collision|EventActorBeginOverlap
  (params (OtherActor :type Actor%20Object%20Reference)))

(event EventTick
  (params (DeltaSeconds :type Float%20%28single-precision%29))
  (Transformation|AddActorWorldOffset (Variables|Default|GetSpeed))
  (if (> (.x (Transformation|GetActorLocation)) 2.5e+03)
    (Variables|Default|SetSpeed (Variables|Default|GetReturnSpeed))
    (elif (< (.x (Transformation|GetActorLocation)) 6.5e+02)
      (Variables|Default|SetSpeed "10.000000, 0, 0"))))

(fn ConstructionScript)